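; Tank pawn that follows path points, aims, fires shells and wears the orange or pink team material taken from its controller.
; Moveby turns the mesh toward the next point, scales speed by yaw cosine to allow reversing, and traces down to align with terrain.
; TransformReplication passes on the resulting transform, applying it only without authority.
; AimBP splits yaw and pitch between turret and gun; ShootBP spawns team-tagged shells.
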(event `self.MoveBy`
  (params (PathPoints :type "Array of Vector Structure (by ref)"))
  (bind _returnvalue (`GameplayStatics.GetWorldDeltaSeconds`))
  (bind (_returnvalue_x _returnvalue_y) (`KismetMathLibrary.BreakVector` (`self.K2_GetActorLocation`)))
  (bind _output (`|GetArrayItem` PathPoints 1))
  (bind _mesh (`self.Mesh`))
  (bind _mesh_2 (`self.Mesh`))
  (bind _returnvalue_2 (`SceneComponent.K2_GetComponentLocation` (`self.Turret`)))
  (bind (_returnvalue_roll _returnvalue_pitch _returnvalue_yaw) (`KismetMathLibrary.BreakRotator` (`KismetMathLibrary.FindRelativeLookAtRotation` (`SceneComponent.K2_GetComponentToWorld` (`self.Mesh`)) _output)))
  (bind _returnvalue_3 (* _returnvalue 100.0 (`KismetMathLibrary.DegCos` _returnvalue_yaw)))
  (`|ExecutionSequence`
    (:`then_0`
      (`SceneComponent.K2_AddLocalRotation` _mesh_2 (`KismetMathLibrary.MakeRotator` 0.0 0.0 (* _returnvalue 100.0 (`KismetMathLibrary.SignOfFloat` _returnvalue_yaw) (`KismetMathLibrary.SelectFloat` 1.0 -1.0 (<= (`KismetMathLibrary.Abs` _returnvalue_yaw) 90.0)))) false false)
      (if (> (`KismetMathLibrary.Vector_Distance2D` (`|GetArrayItem` PathPoints (`KismetArrayLibrary.Array_LastIndex` PathPoints)) (`|GetArrayItem` PathPoints)) _returnvalue_3)
        (`self.K2_AddActorLocalOffset` (* (`SceneComponent.GetForwardVector` _mesh_2) _returnvalue_3))
        (else
          (`self.K2_SetActorLocation` _output)
          (set `self.HasValidDestination` false))))
    (:`then_1`
      (bind _outhit (`KismetSystemLibrary.LineTraceSingleForObjects` _returnvalue_2 (- _returnvalue_2 (0.0 0.0 50.0)) (`|MakeArray` "ObjectTypeQuery1" :!type "EObjectTypeQuery Enum")))
      (bind (_bblockinghit _binitialoverlap _time _distance _location _impactpoint _normal) (`GameplayStatics.BreakHitResult` _outhit))
      (if _bblockinghit
        (`SceneComponent.K2_SetWorldRotation` _mesh (`KismetMathLibrary.MakeRotFromZX` _normal (`SceneComponent.GetForwardVector` _mesh)) false false)
        (`self.K2_SetActorLocation` (`KismetMathLibrary.MakeVector` _returnvalue_x _returnvalue_y (.z _location)))))
    (:`then_2`
      (`self.TransformReplication` (`self.K2_GetActorLocation`) (`SceneComponent.K2_GetComponentRotation` (`self.Mesh`))))))

(event `self.ReceiveBeginPlay`
  (`PrimitiveComponent.SetMaterial` (`self.Body`) 0 (select `bool` (`self.TeamOrange`) :`false` "/Game/TankU/Materials/Team_Pink.Team_Pink" :`true` "/Game/TankU/Materials/Team_Orange.Team_Orange" :!type "MaterialInterface Object Reference") :!label _label))

(event `SetupTeam`
  (goto _label))

(event `self.ReceivePossessed`
  (params (NewController :type "Controller Object Reference"))
  (set `self.TeamOrange` (`Tank_PC_Base.TeamOrange` (cast `/Game/TankU/Blueprints/Tank_PC` NewController :!pure true)))
  (`self.SetupTeam`))

(event `TransformReplication`
  (params (Location :type "Vector Structure") (MeshRotation :type "Rotator Structure"))
  (`/Engine/EditorBlueprintResources/ActorMacros.Switch Has Authority`
    (:`Remote`
      (`self.K2_SetActorLocation` Location)
      (`SceneComponent.K2_SetWorldRotation` (`self.Mesh`) MeshRotation false false))))

(event `self.Shoot_BP`
  (bind (_returnvalue_location _returnvalue_rotation) (`KismetMathLibrary.BreakTransform` (`SceneComponent.K2_GetComponentToWorld` (`self.BulletSpawnLocation`))))
  (`|SpawnActorFromClass` "/Game/TankU/Blueprints/TankShell_BP.TankShell_BP_C" (`KismetMathLibrary.MakeTransform` _returnvalue_location _returnvalue_rotation (0.5 0.5 0.5)) "AlwaysSpawn" "OverrideRootScale" null (`self.TeamOrange`) self))

(event `self.Aim_BP`
  (params (Direction :type "Vector Structure"))
  (bind (_returnvalue_roll _returnvalue_pitch _returnvalue_yaw) (`KismetMathLibrary.BreakRotator` (`KismetMathLibrary.FindRelativeLookAtRotation` (`SceneComponent.K2_GetComponentToWorld` (`self.GunPosition`)) (+ Direction (0.0 0.0 15.0)))))
  (`SceneComponent.K2_AddLocalRotation` (`self.TurretScene`) (`KismetMathLibrary.MakeRotator` 0.0 0.0 _returnvalue_yaw) false false)
  (`SceneComponent.K2_AddLocalRotation` (`self.GunPosition`) (`KismetMathLibrary.MakeRotator` 0.0 _returnvalue_pitch) false false))

(fn `UserConstructionScript`
  (`PrimitiveComponent.SetMaterial` (`self.Body`) 0 (select `bool` (`self.TeamOrange`) :`false` "/Game/TankU/Materials/Team_Pink.Team_Pink" :`true` "/Game/TankU/Materials/Team_Orange.Team_Orange" :!type "MaterialInterface Object Reference")))